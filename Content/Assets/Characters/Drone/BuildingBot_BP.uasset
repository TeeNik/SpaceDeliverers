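; Drone character that travels to a build destination, shows timed build progress and then returns home.
; OnBuildBP chains AI MoveTo to the destination, plays the ProgressWidget animation for the given duration, hides the widget and moves to Home, where it calls OnReturnToHome.
; Tick rotates the widget component to face the first player's camera.
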(event `self.ReceiveTick`
  (params (DeltaSeconds :type "Float (single-precision)"))
  (bind _widget (`self.Widget`))
  (`SceneComponent.K2_SetWorldRotation` _widget (`KismetMathLibrary.FindLookAtRotation` (`SceneComponent.K2_GetComponentLocation` _widget) (`self.K2_GetActorLocation` (`PlayerController.PlayerCameraManager` (`GameplayStatics.GetPlayerController` 0)))) false false))

(event `self.OnBuildBP`
  (params (dest :type "Actor Object Reference") (duration :type "Float (single-precision)"))
  (bind _returnvalue (`AIBlueprintHelperLibrary.GetAIController` self))
  (`AITask_MoveTo.AIMoveTo` _returnvalue (0.0 0.0 0.0) dest
    (:`OnMoveFinished`
      (bind _asprogress_widget (cast `/Game/Assets/HUD/ProgressWidget` (`WidgetComponent.GetUserWidgetObject` (`self.Widget`))))
      (`/Game/Assets/HUD/ProgressWidget.PlayProgressAnimation` _asprogress_widget duration)
      (`KismetSystemLibrary.Delay` duration)
      (`Widget.SetVisibility` _asprogress_widget "Hidden")
      (`AITask_MoveTo.AIMoveTo` _returnvalue (0.0 0.0 0.0) (`self.Home`)
        (:`OnMoveFinished`
          (`self.OnReturnToHome`))))))

(fn `UserConstructionScript`)