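; Enemy bot Blueprint that moves to the first Destructible actor found and attacks it in timed stages.
; On arrival it plays a camera-facing progress widget and sends reached, crash and destroy interface messages, with later stages gated by IsDestroying.
; When it hits a character, OnBotHit freezes their movement for a duration, restores walking, then explodes and destroys the bot.
; Spawning uses timelines to scale a particle and drive a material transition.
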(event `self.ReceiveTick`
  (params (DeltaSeconds :type "Float (single-precision)"))
  (bind _widgetcomponent (`self.WidgetComponent`))
  (`SceneComponent.K2_SetWorldRotation` _widgetcomponent (`KismetMathLibrary.FindLookAtRotation` (`SceneComponent.K2_GetComponentLocation` _widgetcomponent) (`self.K2_GetActorLocation` (`PlayerController.PlayerCameraManager` (`GameplayStatics.GetPlayerController` 0)))) false false))

(event `self.OnBotHit`
  (params (character :type "Character Object Reference") (duration :type "Float (single-precision)"))
  (bind _charactermovement (`Character.CharacterMovement` character))
  (`MovementComponent.StopMovementImmediately` _charactermovement)
  (`CharacterMovementComponent.DisableMovement` _charactermovement)
  (`KismetSystemLibrary.Delay` duration)
  (`CharacterMovementComponent.SetMovementMode` _charactermovement "MOVE_Walking" 0)
  (`GameplayStatics.SpawnEmitterAtLocation` (`self.ExplosionParticle`) (`self.K2_GetActorLocation`) (struct) (`self.ParticleSize`))
  (`self.K2_DestroyActor`))

(event `self.ReceiveBeginPlay`
  (bind _isdestroying (`self.IsDestroying`))
  (bind _timetocrash (`self.TimeToCrash`))
  (bind _timetodestroy (`self.TimeToDestroy`))
  (bind _outactors (`GameplayStatics.GetAllActorsWithInterface` "/Script/SpaceDeliverers.Destructible"))
  (bind _output (`|GetArrayItem` _outactors))
  (`AITask_MoveTo.AIMoveTo` (`AIBlueprintHelperLibrary.GetAIController` self) (`self.K2_GetActorLocation`) _output 10.0
    (:`OnMoveFinished`
      (`self.OnTargetReached` _output)
      (message `Destructible.OnTargetReached` _output)
      (bind _asprogress_widget (cast `/Game/Assets/HUD/ProgressWidget` (`WidgetComponent.GetUserWidgetObject` (`self.WidgetComponent`))))
      (`/Game/Assets/HUD/ProgressWidget.PlayProgressAnimation` _asprogress_widget (+ _timetocrash _timetodestroy))
      (`KismetSystemLibrary.Delay` _timetocrash)
      (if (not _isdestroying)
        (message `Destructible.OnCrashReached` _output)
        (`KismetSystemLibrary.Delay` _timetodestroy)
        (if (not _isdestroying)
          (message `Destructible.OnDestroyReached` _output)
          (`Widget.SetVisibility` _asprogress_widget "Hidden"))))))

(event `self.OnSpawnBP`
  (set `self.ParticleScale` (`SceneComponent.K2_GetComponentScale` (`self.SpawnParticle`)))
  (bind (_direction _scale) (`Timeline|Circle`)
    (:`Update`
      (`SceneComponent.SetRelativeScale3D` (`self.SpawnParticle`) (* (`self.ParticleScale`) _scale))
      (bind (_direction_2 _scale_2) (`Timeline|Timeline_0`)
        (:`Update`
          (`MeshComponent.SetScalarParameterValueOnMaterials` (`self.Mesh`) "Transition" _scale_2))))))

(fn `UserConstructionScript`)