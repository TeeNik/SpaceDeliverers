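; Gem_BP is a collectible mineral gem interactible with animated spawn and collection effects.
; On spawn, a timeline moves it from the spawn location using X and Y offsets and a Height-scaled Z curve, without sweeping.
; On collect, another timeline drives uniform actor scale, then destroys the gem when finished.
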(event `self.OnCollect`
  (bind (_direction _newtrack_0) (`Timeline|Timeline_0`)
    (:`Update`
      (`self.SetActorScale3D` (`KismetMathLibrary.Conv_DoubleToVector` _newtrack_0)))
    (:`Finished`
      (`self.K2_DestroyActor`))))

(event `self.OnPlaySpawnAnimation`
  (params (spawnLocation :type "Vector Structure") (x :type "Float (single-precision)") (y :type "Float (single-precision)"))
  (bind (_direction _z _xy) (`Timeline|Timeline_1` :!via `PlayFromStart`)
    (:`Update`
      (`self.K2_SetActorLocation` (+ spawnLocation (`KismetMathLibrary.MakeVector` (* x _xy) (* y _xy) (* (`self.Height`) _z)))))))

(fn `UserConstructionScript`)