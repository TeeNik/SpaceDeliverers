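; Mineral interactible that releases three gems in timed succession when it is hit.
; OnMineralHit waits briefly, then chains delays between SpawnGem calls, restarting a shared timeline after each spawn.
; The timeline animates the mesh's world scale as a multiple of the relative scale cached at BeginPlay.
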(event `self.ReceiveBeginPlay`
  (set `self.InitialScale` (`SceneComponent.RelativeScale3D` (`self.Mesh`))))

(event `self.OnMineralHit`
  (`KismetSystemLibrary.Delay` 0.6)
  (`self.SpawnGem`)
  (`|ExecutionSequence`
    (:`then_0`
      (bind (_direction _newtrack_0) (`Timeline|Timeline_2` :!via `PlayFromStart` :!label _label)
        (:`Update`
          (`SceneComponent.SetWorldScale3D` (`self.Mesh`) (* (`self.InitialScale`) _newtrack_0)))))
    (:`then_1`
      (`KismetSystemLibrary.Delay` 1.51)
      (`self.SpawnGem`)
      (`|ExecutionSequence`
        (:`then_0`
          (goto _label :!via `PlayFromStart`))
        (:`then_1`
          (`KismetSystemLibrary.Delay` 1.51)
          (`self.SpawnGem`)
          (goto _label :!via `PlayFromStart`))))))

(fn `UserConstructionScript`)