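; Player-controlled turret that aims with look input and disintegrates once its ammo runs out.
; Turn and LookUp axes feed controller yaw and inverted pitch.
; OnAmmoEnd plays a timeline that drives the mesh materials' "Desintegration" scalar, then destroys the actor.
; Leftover yaw-limiting experiments are unwired and never run, so this graph applies no rotation clamp.
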(event `InputAxis|Turn`
  (params (AxisValue :type "Float (single-precision)"))
  (`self.AddControllerYawInput` AxisValue))

(event `InputAxis|LookUp`
  (params (AxisValue :type "Float (single-precision)"))
  (`self.AddControllerPitchInput` (* -1 AxisValue)))

(event `self.OnAmmoEnd`
  (bind (_direction _newtrack_0) (`Timeline|Timeline_0`)
    (:`Update`
      (`MeshComponent.SetScalarParameterValueOnMaterials` (`self.Mesh`) "Desintegration" _newtrack_0))
    (:`Finished`
      (`self.K2_DestroyActor`))))

(fn `UserConstructionScript`)