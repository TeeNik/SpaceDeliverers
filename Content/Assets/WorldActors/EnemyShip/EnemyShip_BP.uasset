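; EnemyShip_BP is an enemy ship actor that plays a portal spawn-in effect and flashes when damaged.
; OnSpawn hides the ship at zero scale and spawns a portal particle, then a timeline scales both up.
; When that finishes, movement starts and a second timeline animates the portal's scale.
; Taking damage on the HealthComponent replays a Blink timeline that drives the mesh's BlinkValue material parameter.
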(event `self.OnSpawn`
  (set `self.InitialScale` (`self.GetActorScale3D`))
  (`self.SetActorScale3D` (0.0 0.0 0.0))
  (bind _returnvalue (`GameplayStatics.SpawnEmitterAtLocation` "/Game/FXVarietyPack/Particles/P_ky_portal.P_ky_portal" (`self.K2_GetActorLocation`) (struct :`Roll` 90.0) (0.0 0.0 0.0) false))
  (bind (_direction _scale) (`Timeline|Timeline_0` :!via `PlayFromStart`)
    (:`Update`
      (`self.SetActorScale3D` (* (`self.InitialScale`) _scale))
      (`SceneComponent.SetWorldScale3D` _returnvalue (* (`KismetMathLibrary.MakeVector` 3.0 3.0 1.0) _scale)))
    (:`Finished`
      (`self.StartMovement`)
      (bind (_direction_2 _scale_2) (`Timeline|Timeline_1`)
        (:`Update`
          (`SceneComponent.SetWorldScale3D` _returnvalue (* (`KismetMathLibrary.MakeVector` 3.0 3.0 1.0) _scale_2)))))))

(event `self.HealthComponent.OnTakeDamage`
  (params (Health :type Integer) (Component :type "HealthComponent Object Reference"))
  (bind (_direction _blink) (`Timeline|Blink` :!via `PlayFromStart`)
    (:`Update`
      (`MeshComponent.SetScalarParameterValueOnMaterials` (`self.Mesh`) "BlinkValue" _blink))))

(fn `UserConstructionScript`)