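; Turret pawn Blueprint that lets a player aim by feeding look input into controller rotation.
; The Turn axis drives controller yaw, and the LookUp axis drives inverted controller pitch.
; Unconnected leftover nodes sketch a clamped local yaw rotation and a yaw-range snap with a debug print, but neither runs.
; The construction script is empty.
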(event `InputAxis|Turn`
  (params (AxisValue :type "Float (single-precision)"))
  (`self.AddControllerYawInput` AxisValue))

(event `InputAxis|LookUp`
  (params (AxisValue :type "Float (single-precision)"))
  (`self.AddControllerPitchInput` (* -1 AxisValue)))

(fn `UserConstructionScript`)